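; BP_Enemy is an enemy actor that reacts to overlaps with the player and with projectiles.
; Touching a BP_Player calls that player's HandleCollision.
; A BP_Projectile hit destroys the projectile, increments the first player pawn's Score, writes it to that player's score widget label, then destroys the enemy.
; All logic runs from ActorBeginOverlap; BeginPlay, Tick and the construction script are empty.
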(event `self.ReceiveActorBeginOverlap`
  (params (OtherActor :type "Actor Object Reference"))
  (bind _asbp_player (cast `/Game/InfiniteMatrix/Blueprints/BP_Player` OtherActor)
    (:`then`
      (`/Game/InfiniteMatrix/Blueprints/BP_Player.HandleCollision` _asbp_player))
    (:`CastFailed`
      (bind _asbp_projectile (cast `/Game/InfiniteMatrix/Blueprints/BP_Projectile` OtherActor))
      (`self.K2_DestroyActor` _asbp_projectile)
      (bind _asbp_player_2 (cast `/Game/InfiniteMatrix/Blueprints/BP_Player` (`GameplayStatics.GetPlayerPawn` 0)))
      (bind _output_get (set `/Game/InfiniteMatrix/Blueprints/BP_Player.Score` (+ (`/Game/InfiniteMatrix/Blueprints/BP_Player.Score` _asbp_player_2) 1) _asbp_player_2))
      (set `/Game/InfiniteMatrix/UI/WBP_Score.Label` (`KismetTextLibrary.Conv_IntToText` _output_get) (`/Game/InfiniteMatrix/Blueprints/BP_Player.ScoreWidget` _asbp_player_2))
      (`self.K2_DestroyActor`))))

(fn `UserConstructionScript`)