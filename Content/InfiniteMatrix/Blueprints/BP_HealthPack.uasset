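; BP_HealthPack is a pickup that restores a fixed amount of the player's health.
; When BP_Player overlaps its Cube component, it adds health capped at MaxHealth, destroys itself and plays a 2D click sound.
; A separate RandomizePack function teleports the static mesh component up by a random Z offset, but nothing in this Blueprint calls it.
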(event `self.Cube.OnComponentBeginOverlap`
  (params (OverlappedComponent :type "PrimitiveComponent Object Reference") (OtherActor :type "Actor Object Reference") (OtherComp :type "PrimitiveComponent Object Reference") (OtherBodyIndex :type Integer) (bFromSweep :type Boolean) (SweepResult :type "HitResult Structure (by ref)"))
  (bind _asbp_player (cast `/Game/InfiniteMatrix/Blueprints/BP_Player` OtherActor))
  (set `/Game/InfiniteMatrix/Blueprints/BP_Player.PlayerHealth` (`KismetMathLibrary.FMin` (+ (`/Game/InfiniteMatrix/Blueprints/BP_Player.PlayerHealth` _asbp_player) 12.5) (`/Game/InfiniteMatrix/Blueprints/BP_Player.MaxHealth` _asbp_player)) _asbp_player)
  (`self.K2_DestroyActor` self)
  (`GameplayStatics.PlaySound2D` "/Engine/VREditor/Sounds/UI/Click_on_Button.Click_on_Button" 0.8 1.0 0.0 null null))

(fn `RandomizePack`
  (`SceneComponent.K2_AddLocalOffset` (`self.StaticMeshComponent`) (`KismetMathLibrary.MakeVector` 0.0 0.0 (`KismetMathLibrary.RandomFloatInRange` 1.0 1000.0)) false true))

(fn `UserConstructionScript`)